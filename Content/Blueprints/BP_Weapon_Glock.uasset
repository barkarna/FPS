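; Glock weapon for the first-person player, handling firing, ammo, dry fire and timed reloading.
; Fire traces from the camera with random spread, then spawns a bullet decal and a cosmetic-style tracer without applying damage.
; Shots play randomized gunshot audio, gun animation, hip or aim-down-sights arm montages, and a brief randomized muzzle flash.
; Reload uses a DoOnce and delay to block firing, refill ammo and toggle the character's reload state.
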(event `self.Fire`
  (bind _asbp_first_person_character (cast `/Game/FirstPerson/Blueprints/BP_FirstPersonCharacter` (`GameplayStatics.GetPlayerCharacter` 0) :!pure true))
  (bind _firstpersonmesh (`/Game/FirstPerson/Blueprints/BP_FirstPersonCharacter.FirstPersonMesh` _asbp_first_person_character))
  (if (`self.ReloadCheck`)
    (if (> (`self.AmmoCount`) 0)
      (`self.AmmoCheck`)
      (bind (_startloc _impactpoint) (`self.LineTrace`))
      (`self.SpawnDecalTracer` _startloc _impactpoint _impactpoint)
      (if (`/Game/FirstPerson/Blueprints/BP_FirstPersonCharacter.AimDown` _asbp_first_person_character)
        (`|PlayMontage` _firstpersonmesh "/Game/Weapon/Glock/ArmsAnim/AM_Glock_ADS.AM_Glock_ADS"
          (:`then`
            _))
        (else
          (`|PlayMontage` _firstpersonmesh "/Game/Weapon/Glock/ArmsAnim/AM_GlockArms.AM_GlockArms"
            (:`then`
              _))))
      (`self.Flash`)
      (else
        (`GameplayStatics.PlaySoundAtLocation` "/Game/Weapon/Sounds/DryFire.DryFire" (`self.K2_GetActorLocation`) (struct) 1.0 1.0 0.0 "/Game/Weapon/Sounds/SA_Shoot.SA_Shoot" "/Game/Weapon/Sounds/SC_Shoot.SC_Shoot" null null)))))

(event `self.Reload`
  (bind _asbp_first_person_character (cast `/Game/FirstPerson/Blueprints/BP_FirstPersonCharacter` (`GameplayStatics.GetPlayerCharacter` 0) :!pure true))
  (if (< (`self.AmmoCount`) (`self.MaxAmmo`))
    (`/Engine/EditorBlueprintResources/StandardMacros.DoOnce` false :!label _label
      (:`Completed`
        (set `/Game/FirstPerson/Blueprints/BP_FirstPersonCharacter.IsReload` true _asbp_first_person_character)
        ;[1 1 1] OR
        (`AnimInstance.Montage_Play` (`SkeletalMeshComponent.GetAnimInstance` (`/Game/FirstPerson/Blueprints/BP_FirstPersonCharacter.FirstPersonMesh` _asbp_first_person_character)) "/Game/Weapon/Glock/ArmsAnim/AM_GlockReload.AM_GlockReload" 1.0 "MontageLength" 0.0 true)
        (`SkeletalMeshComponent.PlayAnimation` (`self.SkeletalMesh`) "/Game/Weapon/Glock/Glock_Reload_anim.Glock_Reload_anim" false)
        (set `self.ReloadCheck` false)
        (`KismetSystemLibrary.Delay` (`self.ReloadTime`))
        (set `self.AmmoCount` (`self.MaxAmmo`))
        (set `self.ReloadCheck` true)
        (set `/Game/FirstPerson/Blueprints/BP_FirstPersonCharacter.IsReload` false _asbp_first_person_character)
        (goto _label :!via `Reset`)))))

(fn `AmmoCheck`
  (bind _returnvalue (`KismetMathLibrary.RandomFloatInRange` 0.7 1.2))
  (`/Engine/EditorBlueprintResources/StandardMacros.DecrementInt` (`self.AmmoCount`)
    (:`  `
      (`GameplayStatics.PlaySoundAtLocation` "/Game/Weapon/Sounds/Gunshot.Gunshot" (`self.K2_GetActorLocation`) (struct) (* _returnvalue 1.5) _returnvalue 0.0 "/Game/Weapon/Sounds/SA_Shoot.SA_Shoot" "/Game/Weapon/Sounds/SC_Shoot.SC_Shoot" null null)
      (`SkeletalMeshComponent.PlayAnimation` (`self.SkeletalMesh`) "/Game/Weapon/Glock/Glock_Fire_anim.Glock_Fire_anim" false))))

(fn `LineTrace`
  (returns (StartLoc :type "Vector Structure") (ImpactPoint :type "Vector Structure"))
  (bind _bulletspray (`self.BulletSpray`))
  (bind _returnvalue (`SceneComponent.K2_GetComponentLocation` (`self.Scene`)))
  (bind _returnvalue_2 (* _bulletspray -1.0))
  (bind _firstpersoncamera (`/Game/FirstPerson/Blueprints/BP_FirstPersonCharacter.FirstPersonCamera` (cast `/Game/FirstPerson/Blueprints/BP_FirstPersonCharacter` (`GameplayStatics.GetPlayerCharacter` 0) :!pure true)))
  (bind _returnvalue_3 (`SceneComponent.K2_GetComponentLocation` _firstpersoncamera))
  (bind _outhit (`KismetSystemLibrary.LineTraceSingle` _returnvalue_3 (+ (+ _returnvalue_3 (* (`SceneComponent.GetForwardVector` _firstpersoncamera) 20000.0)) (`KismetMathLibrary.MakeVector` (`KismetMathLibrary.RandomFloatInRange` _returnvalue_2 _bulletspray) (`KismetMathLibrary.RandomFloatInRange` _returnvalue_2 _bulletspray) (`KismetMathLibrary.RandomFloatInRange` _returnvalue_2 _bulletspray))) "TraceTypeQuery1"))
  (bind (_bblockinghit _binitialoverlap _time _distance _location _impactpoint) (`GameplayStatics.BreakHitResult` _outhit))
  (`KismetSystemLibrary.LineTraceSingle` :`Start` _returnvalue :`End` _impactpoint :`TraceChannel` "TraceTypeQuery1" :`TraceColor` (struct :`R` 0.17946 :`G` 0.890222 :`B` 1.0 :`A` 1.0))
  (return _returnvalue _impactpoint))

(fn `SpawnDecalTracer`
  (params (Location :type "Vector Structure") (SpawnTransform :type "Vector Structure") (ImpactPoint :type "Vector Structure"))
  (`GameplayStatics.SpawnDecalAtLocation` "/Game/Materials/M_BulletDecal.M_BulletDecal" (10.0 10.0 10.0) SpawnTransform (`KismetMathLibrary.Conv_VectorToRotator` ImpactPoint) 10.0)
  (if (>= (`KismetMathLibrary.RandomIntegerInRange` 0) 0)
    (`|SpawnActorFromClass` "/Game/Blueprints/BP_Tracer.BP_Tracer_C" (`KismetMathLibrary.MakeTransform` Location (`SceneComponent.K2_GetComponentRotation` (`/Game/FirstPerson/Blueprints/BP_FirstPersonCharacter.FirstPersonCamera` (cast `/Game/FirstPerson/Blueprints/BP_FirstPersonCharacter` (`GameplayStatics.GetPlayerCharacter` 0) :!pure true))) (0.1 0.1 0.1)) "Undefined" "MultiplyWithRoot" null null)
    (return)))

(fn `UserConstructionScript`
  (`parent.UserConstructionScript`)
  (set `self.MaxAmmo` 7)
  (set `self.AmmoCount` 7)
  (set `self.ReloadTime` 1.5)
  (set `self.BulletSpray` 500.0)
  (set `self.ReloadTime` 1.8))